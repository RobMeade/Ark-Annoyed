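; Game mode for ArkAnnoyed that handles moving to the next level when one is completed.
; LevelComplete gets the next level index from the game instance through a message call and opens that entry in the Levels array by name.
; An index past the end of the array opens TitleScreen instead.
; GetNextLevel and GetPersistantData are stubs here that return zero for level, lives and score.
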(event `/Game/ArkAnnoyed/Game/BPI_GameFramework.LevelComplete`
  (bind _level (message `/Game/ArkAnnoyed/Game/BPI_GameFramework.GetNextLevel` (`GameplayStatics.GetGameInstance`)))
  (if (< _level (`KismetArrayLibrary.Array_Length` (`self.Levels`)))
    (`GameplayStatics.OpenLevel` (`|GetArrayItem` (`self.Levels`) _level))
    (else
      (`GameplayStatics.OpenLevel` "TitleScreen"))))

(fn `GetNextLevel`
  (returns (Level :type Integer))
  (return 0))

(fn `GetPersistantData`
  (returns (Lives :type Integer) (Score :type Integer))
  (return 0 0))

(fn `UserConstructionScript`)