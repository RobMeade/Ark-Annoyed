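; Player controller for the paddle in ArkAnnoyed that turns horizontal Enhanced Input into paddle movement.
; It registers the default mapping context on BeginPlay and caches the possessed BP_Paddle.
; The move axis, scaled by a speed multiplier, picks right, left or stop by sign and feeds the paddle's movement play rate.
; Releasing the input stops the paddle.
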(event `self.ReceiveBeginPlay`
  (bind _returnvalue (pcsubsystem `EnhancedInputLocalPlayerSubsystem` self))
  (`/Engine/EditorBlueprintResources/StandardMacros.IsValid` _returnvalue
    (:`Is Valid`
      (`EnhancedInputSubsystemInterface.AddMappingContext` _returnvalue "/Game/ArkAnnoyed/Player/Input/IMC_Default.IMC_Default" 0 (struct)))
    (:`Is Not Valid`
      (`KismetSystemLibrary.PrintString` "Enhanced Input Local Player Subsystem Not Found"))))

(event `self.ReceivePossess`
  (params (PossessedPawn :type "Pawn Object Reference"))
  (bind _asbp_paddle (cast `/Game/ArkAnnoyed/Player/BP_Paddle` PossessedPawn)
    (:`then`
      (set `self.Paddle` _asbp_paddle))
    (:`CastFailed`
      (`KismetSystemLibrary.PrintString` "Cast of Pawn to BP_Paddle Failed"))))

(event `EnhancedInput|/Game/ArkAnnoyed/Player/Input/IA_MoveHorizontally`
  (params (ActionValue :type "Vector2D Structure") (ElapsedSeconds :type "Float (double-precision)") (TriggeredSeconds :type "Float (double-precision)") (InputAction :type "InputAction Object Reference" :default "/Game/ArkAnnoyed/Player/Input/IA_MoveHorizontally.IA_MoveHorizontally"))
  (bind _paddle (`self.Paddle`))
  (:`Triggered`
    (bind _output_get (set `self.MoveRate` (* ActionValue_X (`self.PaddleSpeedMultiplier`))))
    (`/Engine/EditorBlueprintResources/StandardMacros.CompareFloat` _output_get
      (:`>`
        (`/Game/ArkAnnoyed/Player/BP_Paddle.MoveRight` _paddle)
        (`/Game/ArkAnnoyed/Player/BP_Paddle.SetMovePaddlePlayRate` (`self.Paddle`) (`self.MoveRate`) :!label _label))
      (:`==`
        (`/Game/ArkAnnoyed/Player/BP_Paddle.StopMoving` _paddle :!label _label_2))
      (:`<`
        (`/Game/ArkAnnoyed/Player/BP_Paddle.MoveLeft` _paddle)
        (`/Engine/EditorBlueprintResources/StandardMacros.NegateFloat` (`self.MoveRate`)
          (:`  `
            (goto _label))))))
  (:`Completed`
    (goto _label_2)))

(fn `UserConstructionScript`)