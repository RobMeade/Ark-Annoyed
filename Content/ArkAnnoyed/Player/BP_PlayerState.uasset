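; Player state for the ArkAnnoyed brick-breaker, tracking lives, score and remaining brick count.
; On BeginPlay it restores lives and score from the GameInstance and pushes them to the player controller through message calls.
; Score and life changes notify the controller, life changes also notify the pawn, and running out of lives opens the title screen.
; When the last brick is destroyed it saves lives and score to the GameInstance and signals level completion to the GameMode.
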(event `self.ReceiveBeginPlay`
  (bind (_lives _score) (message `/Game/ArkAnnoyed/Game/BPI_GameFramework.GetPersistantData` (`GameplayStatics.GetGameInstance`)))
  (set `self.CurrentLives` _lives)
  (set `self.CurrentScore` _score)
  (message `/Game/ArkAnnoyed/Game/BPI_GameFramework.UpdateLives` (`self.GetPlayerController`) (`self.CurrentLives`))
  (message `/Game/ArkAnnoyed/Game/BPI_GameFramework.UpdateScore` (`self.GetPlayerController`) (`self.CurrentScore`)))

(event `/Game/ArkAnnoyed/Game/BPI_GameFramework.UpdateScore`
  (params (Points :type Integer))
  (set `self.CurrentScore` (+ Points (`self.CurrentScore`)))
  (message `/Game/ArkAnnoyed/Game/BPI_GameFramework.UpdateScore` (`self.GetPlayerController`) (`self.CurrentScore`)))

(event `/Game/ArkAnnoyed/Game/BPI_GameFramework.UpdateLives`
  (params (Lives :type Integer))
  (bind _output_get (set `self.CurrentLives` (+ Lives (`self.CurrentLives`))))
  (if (< _output_get 1)
    (`GameplayStatics.OpenLevel` "TitleScreen")
    (else
      (message `/Game/ArkAnnoyed/Game/BPI_GameFramework.UpdateLives` (`GameplayStatics.GetPlayerPawn` 0) (`self.CurrentLives`))
      (message `/Game/ArkAnnoyed/Game/BPI_GameFramework.UpdateLives` (`self.GetPlayerController`) (`self.CurrentLives`)))))

(event `/Game/ArkAnnoyed/Game/BPI_GameFramework.UpdateBrickCount`
  (params (Bricks :type Integer))
  (set `self.BrickCount` (+ Bricks (`self.BrickCount`))))

(event `/Game/ArkAnnoyed/Game/BPI_GameFramework.BrickDestroyed`
  (bind _result (`/Engine/EditorBlueprintResources/StandardMacros.DecrementInt` (`self.BrickCount`))
    (:`  `
      (if (<= _result 0)
        (message `/Game/ArkAnnoyed/Game/BPI_GameFramework.SetPersistantData` (`GameplayStatics.GetGameInstance`) (`self.CurrentLives`) (`self.CurrentScore`))
        (message `/Game/ArkAnnoyed/Game/BPI_GameFramework.LevelComplete` (`GameplayStatics.GetGameMode`))))))

(fn `GetNextLevel`
  (returns (Level :type Integer))
  (return 0))

(fn `GetPersistantData`
  (returns (Lives :type Integer) (Score :type Integer))
  (return 0 0))

(fn `UserConstructionScript`)