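; BP_BrickSpawner lays out the grid of bricks for the level and reports the brick count to the player state.
; The construction script derives column and row counts from WidgetPosition's X and Z divided by cell size.
; A self-re-entering DoN node, reset after each row, acts as a nested loop adding BP_Brick_Base child actor components on a fixed Y plane.
; BeginPlay passes the child actor count to UpdateBrickCountMessage.
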(event `self.ReceiveBeginPlay`
  (message `/Game/ArkAnnoyed/Game/BPI_GameFramework.UpdateBrickCount` (`GameplayStatics.GetPlayerState` 0) (`KismetArrayLibrary.Array_Length` (`self.GetAllChildActors` true))))

(fn `UserConstructionScript`
  (bind (_widgetposition_x _widgetposition_y _widgetposition_z) (`KismetMathLibrary.BreakVector` (`self.WidgetPosition`)))
  (set `self.ColumnCount` (`KismetMathLibrary.FTrunc` (/ _widgetposition_x (`self.ColumnWidth`))))
  (set `self.RowCount` (`KismetMathLibrary.FTrunc` (/ _widgetposition_z (`self.RowHeight`))))
  (bind _counter (`/Engine/EditorBlueprintResources/StandardMacros.Do N` (`self.ColumnCount`) :!label _label)
    (:`Exit`
      (bind _returnvalue (`AddComponent|NODE_AddChildActorComponent-0` :`RelativeTransform` (`KismetMathLibrary.MakeTransform` (`KismetMathLibrary.MakeVector` (`self.WorkingColumnPosition`) (`self.PlanePosition`) (`self.WorkingRowPosition`)))))
      (`ChildActorComponent.SetChildActorClass` _returnvalue "/Game/ArkAnnoyed/Environment/Brick/BP_Brick_Base.BP_Brick_Base_C")
      (if (>= _counter (`self.ColumnCount`))
        (bind _result (`/Engine/EditorBlueprintResources/StandardMacros.IncrementInt` (`self.WorkingRowCount`))
          (:`  `
            (if (not (>= _result (`self.RowCount`)))
              (set `self.WorkingRowPosition` (+ (`self.RowHeight`) (`self.WorkingRowPosition`)))
              (set `self.WorkingColumnPosition` (`self.DefaultColumnPosition`))
              (`|ExecutionSequence`
                (:`then_0`
                  (goto _label :!via `Reset`))
                (:`then_1`
                  (goto _label))))))
        (else
          (set `self.WorkingColumnPosition` (+ (`self.ColumnWidth`) (`self.WorkingColumnPosition`)))
          (goto _label))))))